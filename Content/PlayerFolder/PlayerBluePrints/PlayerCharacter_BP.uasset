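; Player character Blueprint for what appears to be a survival game, handling movement, handheld items and death.
; Pickup flags gate the flashlight and map toggles and the journal, which opens a widget.
; Shift sprints, C toggles crouch, and jumping drains StatsComp stamina through a timeline lerp.
; Journal and death screens halt movement and switch to UI-only input, while PlayerStart restores game control on BeginPlay.
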(event EventBeginPlay
  (CallFunction|PlayerStart))

(event EventOnMapPress
  ;[1 1 1] M Key   (Map)
  (if (Variables|Tools|GetPickedUpMap?)
    (Utilities|FlowControl|FlipFlop
      (:A
        (Utilities|FlowControl|DoOnce false :!label _label
          (:Completed
            (Variables|/Script/Engine.PlayerController|SetbShowMouseCursor (Game|GetPlayerController 0) false)
            (Rendering|SetVisibility (Variables|Default|GetBp-Map) true false)
            (Audio|PlaySound2D "/Game/Audio/Map/MapOpen.MapOpen" 1.0 1.0 0.0 0 0))))
      (:B
        (Audio|PlaySound2D "/Game/Audio/Map/MapClose.MapClose" 1.0 1.0 0.0 0 0)
        (Rendering|SetVisibility (Variables|Default|GetBp-Map) false false)
        (goto _label Reset)))))

(event EventOnJournalPress
  (bind _returnvalue (Game|GetPlayerController 0))
  (bind _charactermovement (Variables|Character|GetCharacterMovement))
  ;[1 1 1] J Key (Journal
  (if (Variables|Tools|GetPickedUpJournal?)
    ;;[1 1 1] Comment
    (Rendering|SetVisibility (Variables|Default|GetBp-Map) false false)
    (Rendering|SetVisibility (Variables|Default|GetBP-Journal) true false)
    ;;[1 1 1] Comment
    (Audio|PlaySound2D "/Game/Audio/Journal/JournalOpen.JournalOpen" 1.0 1.0 0.0 0 0) ; Journal Open
    ;;[1 1 1] Add Journal Widget
    (bind _returnvalue_2 (CallFunction|CreateWidget "/Game/UI/Journal/WB-Journal.WB-Journal_C"))
    (UserInterface|Viewport|AddtoViewport _returnvalue_2 0)
    ;;[1 1 1] Comment
    (Components|Movement|StopMovementImmediately _charactermovement)
    (Pawn|Components|CharacterMovement|SetMovementMode _charactermovement "MOVE_None" 0)
    (Variables|/Script/Engine.PlayerController|SetbShowMouseCursor _returnvalue true)
    (Input|SetInputModeUIOnly _returnvalue _returnvalue_2 "DoNotLock" false)))

(event EventOnFlashlightPress
  (bind _bp_flashlight (Variables|Default|GetBP-Flashlight))
  ;[1 1 1] F Key (Flashlight
  (if (Variables|Tools|GetPickedUpLight?)
    (Utilities|FlowControl|FlipFlop
      (:A
        (Rendering|SetVisibility _bp_flashlight true false)
        (Audio|PlaySoundatLocation "/Game/Audio/Flashlight/Flashlight_1.Flashlight_1" (Transformation|GetWorldLocation (Variables|Default|GetBP-Flashlight)) "0, 0, 0" 1.0 1.0 0.0 0 0 0 0))
      (:B
        (Rendering|SetVisibility _bp_flashlight false false)
        (Audio|PlaySoundatLocation "/Game/Audio/Flashlight/Flashlight_2.Flashlight_2" "0, 0, 0" "0, 0, 0" 1.0 1.0 0.0 0 0 0 0)))))

(event EventOnJumped
  (bind _statscomp (Variables|Default|GetStatsComp))
  ;[1 1 1] Jump and Crouch
  (bind _returnvalue (Class|StatsComponent|GetCurrentStamina _statscomp))
  (bind _lerpstamina (Timeline|Stamina%20Timeline PlayFromStart)
    (:Update
      (Class|StatsComponent|SetCurrentStamina _statscomp (Math|Float|Truncate (Math|Float|Lerp (Math|Conversions|ToFloat(Integer) _returnvalue) (Math|Conversions|ToFloat(Integer) (- _returnvalue (Variables|PlayerSystems|GetJumpStaminaDrain))) _lerpstamina))))))

(event Input|KeyboardEvents|SpaceBar
  (params (Key :type Key%20Structure :default "None"))
  ;[1 1 1] Jump and Crouch
  (:Pressed
    (Character|Jump)))

(event Input|KeyboardEvents|F
  (params (Key :type Key%20Structure :default "None"))
  ;[1 1 1] F Key (Flashlight
)

(event Input|KeyboardEvents|C
  (params (Key :type Key%20Structure :default "None"))
  ;[1 1 1] Jump and Crouch
  ;;[1 1 1] Crouch
  (:Pressed
    (Utilities|FlowControl|FlipFlop
      (:A
        (Character|Crouch))
      (:B
        (Character|UnCrouch)))))

(event Input|KeyboardEvents|LeftShift
  (params (Key :type Key%20Structure :default "None"))
  (bind _charactermovement (Variables|Character|GetCharacterMovement))
  ;[1 1 1] Jump and Crouch
  (:Pressed
    (Variables|/Script/Engine.CharacterMovementComponent|SetMaxWalkSpeed _charactermovement 8e+02))
  (:Released
    (Variables|/Script/Engine.CharacterMovementComponent|SetMaxWalkSpeed _charactermovement 6e+02)))

(fn ConstructionScript)

(fn DebugPrintStringItems
  (bind _returnvalue (Utilities|Time|GetWorldDeltaSeconds))
  (Development|PrintString (Utilities|String|Append "Bistort Amount:" (Utilities|String|ToString(Integer) 0)) true true "(R=0.000000,G=0.660000,B=1.000000,A=1.000000)" _returnvalue)
  (Development|PrintString (Utilities|String|Append "Dandelion:" (Utilities|String|ToString(Integer) 0)) true true "(R=0.000000,G=0.660000,B=1.000000,A=1.000000)" _returnvalue)
  (Development|PrintString (Utilities|String|Append "Acorn:" (Utilities|String|ToString(Integer) 0)) true true "(R=0.000000,G=0.660000,B=1.000000,A=1.000000)" _returnvalue)
  (Development|PrintString (Utilities|String|Append "Golden Rods:" (Utilities|String|ToString(Integer) 0)) true true "(R=0.000000,G=0.660000,B=1.000000,A=1.000000)" _returnvalue)
  (Development|PrintString (Utilities|String|Append "Asparagus:" (Utilities|String|ToString(Integer) 0)) true true "(R=0.000000,G=0.660000,B=1.000000,A=1.000000)" _returnvalue)
  (Development|PrintString (Utilities|String|Append "Raspberry:" (Utilities|String|ToString(Integer) 0)) true true "(R=0.658375,G=0.000000,B=0.049707,A=1.000000)" _returnvalue)
  (Development|PrintString (Utilities|String|Append "Strawberry:" (Utilities|String|ToString(Integer) 0)) true true "(R=0.657292,G=0.000000,B=0.049450,A=1.000000)" _returnvalue)
  (Development|PrintString (Utilities|String|Append "Blackberry:" (Utilities|String|ToString(Integer) 0)) true true "(R=0.000000,G=0.660000,B=1.000000,A=1.000000)" _returnvalue)
  (Development|PrintString (Utilities|String|Append "Mushroom:" (Utilities|String|ToString(Integer) 0)) true true "(R=0.000000,G=0.660000,B=1.000000,A=1.000000)" _returnvalue)
  (Development|PrintString (Utilities|String|Append "Lethal Mushroom: " (Utilities|String|ToString(Integer) 0)) true true "(R=0.000000,G=0.660000,B=1.000000,A=1.000000)" _returnvalue)
  (Development|PrintString (Utilities|String|Append "Gas Mushroom:" (Utilities|String|ToString(Integer) 0)) true true "(R=0.000000,G=1.000000,B=0.222381,A=1.000000)" _returnvalue)
  (Development|PrintString (Utilities|String|Append "Wood:" (Utilities|String|ToString(Integer) 0)) true true "(R=0.000000,G=0.658375,B=1.000000,A=1.000000)" _returnvalue)
  (Development|PrintString (Utilities|String|Append "Rock:" (Utilities|String|ToString(Integer) 0)) true true "(R=0.000000,G=0.660000,B=1.000000,A=1.000000)" _returnvalue)
  (Development|PrintString (Utilities|String|Append "Clay:" (Utilities|String|ToString(Integer) 0)) true true "(R=0.000000,G=0.660000,B=1.000000,A=1.000000)" _returnvalue)
  (Development|PrintString (Utilities|String|Append "Electronic Component:" (Utilities|String|ToString(Integer) 0)) true true "(R=0.000000,G=1.000000,B=0.188942,A=1.000000)" _returnvalue)
  (Development|PrintString (Utilities|String|Append "Tree Sap:" (Utilities|String|ToString(Integer) 0)) true true "(R=1.000000,G=0.584970,B=0.000000,A=1.000000)" _returnvalue)
  (Development|PrintString (Utilities|String|Append "Wood Fibre:" (Utilities|String|ToString(Integer) (Variables|PlantFibre|GetPlant%20Fibre%20Current))) true true "(R=0.000000,G=0.660000,B=1.000000,A=1.000000)" _returnvalue)
  (Development|PrintString (Utilities|String|Append "Coal:" (Utilities|String|ToString(Integer) 0)) true true "(R=0.000000,G=0.660000,B=1.000000,A=1.000000)" _returnvalue)
  (Development|PrintString (Utilities|String|Append "Iron ore:" (Utilities|String|ToString(Integer) 0)) true true "(R=0.000000,G=0.660000,B=1.000000,A=1.000000)" _returnvalue)
  (Development|PrintString (Utilities|String|Append "Metal Component: " (Utilities|String|ToString(Integer) 0)) true true "(R=0.000000,G=0.660000,B=1.000000,A=1.000000)" _returnvalue)
  (Development|PrintString (Utilities|String|Append "Sticks: " (Utilities|String|ToString(Integer) 0)) true true "(R=0.000000,G=0.660000,B=1.000000,A=1.000000)" _returnvalue)
  (Development|PrintString (Utilities|String|Append "Blueberry:" (Utilities|String|ToString(Integer) 0)) true true "(R=0.000000,G=0.660000,B=1.000000,A=1.000000)" _returnvalue))

(fn PlayerDeath
  (bind _returnvalue (Game|GetPlayerController 0))
  (Components|Movement|StopMovementImmediately (Variables|Character|GetCharacterMovement))
  (Pawn|Components|CharacterMovement|SetMovementMode (Variables|Character|GetCharacterMovement) "MOVE_None" 0)
  (bind _returnvalue_2 (UserInterface|CreateWidget "/Game/UI/WB-PlayerDied.WB-PlayerDied_C"))
  (UserInterface|Viewport|AddtoViewport _returnvalue_2 0)
  (Variables|/Script/Engine.PlayerController|SetbShowMouseCursor _returnvalue true)
  (Input|SetInputModeUIOnly _returnvalue _returnvalue_2 "DoNotLock" false))

(fn PlayerStart
  (bind _returnvalue (Game|GetPlayerController 0))
  (Pawn|Components|CharacterMovement|SetMovementMode (Variables|Character|GetCharacterMovement) "MOVE_Walking" 0)
  (Variables|/Script/Engine.PlayerController|SetbShowMouseCursor _returnvalue false)
  (Input|SetInputModeGameOnly _returnvalue false))

(fn CreateWidget
  (params (Widget :type User%20Widget%20Class%20Reference))
  (bind _returnvalue (UserInterface|CreateWidget Widget))
  (UserInterface|Viewport|AddtoViewport _returnvalue 0)
  (return _returnvalue))

(fn RemoveWidget
  (params (Target :type Widget%20Object%20Reference))
  (Widget|RemovefromParent Target))

(fn WidgetInput
  (bind _returnvalue (Game|GetPlayerController 0))
  (Components|Movement|StopMovementImmediately (Variables|Character|GetCharacterMovement))
  (Pawn|Components|CharacterMovement|SetMovementMode (Variables|Character|GetCharacterMovement) "MOVE_None" 0)
  (Variables|/Script/Engine.PlayerController|SetbShowMouseCursor _returnvalue true)
  (Input|SetInputModeUIOnly _returnvalue 0 "DoNotLock" false))