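; BP_Planter_Single is a farming planter Blueprint that advances with game time.
; After the parent BeginPlay, it binds to the GameTimeManager's OnGameTimePassed event, retrying every 0.2 seconds by fetching that component from the custom game mode until it is valid.
; Each event forwards the elapsed time to TimePassed, with no other planting logic in this graph.
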(event Custom|GameTimePassed
  (params (TimePassed :type Timespan%20Structure) (CurGameTime :type Date%20Time%20Structure))
  (Class|Planter|TimePassed TimePassed))

(event EventBeginPlay
  (|CallParentFunction)
  (Utilities|IsValid (Variables|Default|GetGame%20Time%20Manager) :!label _label
    (:Is%20Valid
      (EventDispatchers|BindEventtoOnGameTimePassed (Variables|Default|GetGame%20Time%20Manager) (delegate Custom|GameTimePassed)))
    (:Is%20Not%20Valid
      (Utilities|FlowControl|Delay 0.2)
      (bind _ascustom_game_mode_base (Utilities|Casting|CastToCustomGameModeBase (Game|GetGameMode)))
      (Variables|Default|SetGame%20Time%20Manager (Actor|GetComponentbyClass _ascustom_game_mode_base "/Script/CozyCabinsGame.GameTimeManager"))
      (goto _label))))

(fn ConstructionScript)