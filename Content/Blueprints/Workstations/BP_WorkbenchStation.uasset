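; Workbench station actor that must be repaired through its ACRepair component before interacting opens its widget.
; Interacting while broken attempts a repair, and success hides the prompt and displays the widget immediately.
; While unrepaired, a Character entering the sphere reveals text of the repair requirements.
; A looping timer turns that text toward the player with clamped pitch until overlap ends or repair succeeds.
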(event OnComponentBeginOverlap(Sphere)
  (params (OverlappedComponent :type Primitive%20Component%20Object%20Reference) (OtherActor :type Actor%20Object%20Reference) (OtherComp :type Primitive%20Component%20Object%20Reference) (OtherBodyIndex :type Integer) (bFromSweep :type Boolean) (SweepResult :type Hit%20Result%20Structure%20%28by%20ref%29))
  (bind _ac_repair (Variables|Default|GetAC_Repair))
  (bind _textrender (Variables|Default|GetTextRender))
  ;[1 1 1] Display Repair Text
  (Utilities|Casting|CastToCharacter OtherActor)
  (if (not (Default|GetRepairStatus _ac_repair))
    (Rendering|Components|TextRender|SetText (Variables|Default|GetTextRender) (Default|ReturnRequiredText _ac_repair))
    (Rendering|SetVisibility _textrender true false)
    (Development|SetHiddeninGame _textrender false false)
    (bind _returnvalue (Utilities|Time|SetTimerbyEvent (delegate Custom|RotateToPlayer) 0.01 true))
    (Variables|Default|SetRotationHandle _returnvalue)))

(event OnComponentEndOverlap(Sphere)
  (params (OverlappedComponent :type Primitive%20Component%20Object%20Reference) (OtherActor :type Actor%20Object%20Reference) (OtherComp :type Primitive%20Component%20Object%20Reference) (OtherBodyIndex :type Integer))
  (bind _textrender (Variables|Default|GetTextRender))
  ;[1 1 1] Display Repair Text
  (Utilities|Casting|CastToCharacter OtherActor)
  (Rendering|SetVisibility _textrender false false)
  (Development|SetHiddeninGame _textrender true false)
  (Utilities|Time|ClearandInvalidateTimerbyHandle (Variables|Default|GetRotationHandle)))

(event Custom|RotateToPlayer
  (bind _returnvalue (Game|GetPlayerCharacter 0))
  (bind _textrender (Variables|Default|GetTextRender))
  (bind _returnvalue_2 (Transformation|GetWorldLocation _textrender))
  (bind _returnvalue_3 (Transformation|GetActorLocation _returnvalue))
  (bind _returnvalue_4 (Math|Rotator|FindLookatRotation _returnvalue_2 _returnvalue_3))
  (bind (_roll _pitch _yaw) (Math|Rotator|BreakRotator _returnvalue_4))
  ;[1 1 1] Rotation
  (Transformation|SetWorldRotation (Variables|Default|GetTextRender) (Math|Rotator|MakeRotator _roll (Math|Float|Clamp(Float) _pitch -2e+01 2e+01) _yaw) false false))

(event Custom|ManualHide
  (bind _textrender (Variables|Default|GetTextRender))
  ;[1 1 1] Display Repair Text
  (Rendering|SetVisibility _textrender false false)
  (Development|SetHiddeninGame _textrender true false)
  (Utilities|Time|ClearandInvalidateTimerbyHandle (Variables|Default|GetRotationHandle)))

(event EventOnInteract
  (params (World :type World%20Object%20Reference) (SourceCharacter :type Character%20Object%20Reference))
  ;[1 1 1] On Hit/Interact
  (if (Default|GetRepairStatus (Variables|Default|GetAC_Repair))
    (Class|WorkStationBase|DisplayWidget World SourceCharacter :!label _label)
    (else
      (bind _success (Default|AttemptRepair (Variables|Default|GetAC_Repair)))
      (if _success
        (CallFunction|ManualHide)
        (goto _label)))))

(fn ConstructionScript)