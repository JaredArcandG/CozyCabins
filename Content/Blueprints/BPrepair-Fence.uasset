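; Repairable fence actor that the player fixes by interacting and spending wood.
; OnInteract checks the player's wood against the cost, then either repairs once (deducts wood, optionally swaps the mesh, disables the trigger box, spawns an effect) or shows a not-enough-resources widget.
; The trigger box toggles a prompt text that turns to face the camera every tick, and clears the widget on overlap end.
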(event OnComponentBeginOverlap(BoxCollision)
  (params (OverlappedComponent :type Primitive%20Component%20Object%20Reference) (OtherActor :type Actor%20Object%20Reference) (OtherComp :type Primitive%20Component%20Object%20Reference) (OtherBodyIndex :type Integer) (bFromSweep :type Boolean) (SweepResult :type Hit%20Result%20Structure%20%28by%20ref%29))
  ;[0 0.846 1] Collision Detection (check if player)
  (if (not (Variables|Default|GetHasBeenFixed?))
    (if (== OtherActor (Game|GetPlayerCharacter 0))
      (Rendering|SetVisibility (Variables|Default|GetTextRender) true false))))

(event OnComponentEndOverlap(BoxCollision)
  (params (OverlappedComponent :type Primitive%20Component%20Object%20Reference) (OtherActor :type Actor%20Object%20Reference) (OtherComp :type Primitive%20Component%20Object%20Reference) (OtherBodyIndex :type Integer))
  ;[0 0.846 1] Collision Detection (check if player)
  (if (not (Variables|Default|GetHasBeenFixed?))
    (Widget|RemovefromParent (Variables|Default|GetWIdgetReferenceNER))
    (if (== OtherActor (Game|GetPlayerCharacter 0))
      (Rendering|SetVisibility (Variables|Default|GetTextRender) false false))))

(event EventTick
  (params (DeltaSeconds :type Float%20%28single-precision%29))
  (bind _textrender (Variables|Default|GetTextRender))
  ;[0 0.8713 1] Testing
  (Transformation|SetWorldRotation _textrender (Math|Rotator|FindLookatRotation (Transformation|GetWorldLocation _textrender) (Transformation|GetWorldLocation (Variables|/Script/Engine.PlayerCameraManager|GetTransformComponent (Game|GetPlayerCameraManager 0)))) false false))

(event EventOnInteract
  (params (World :type World%20Object%20Reference) (SourceCharacter :type Character%20Object%20Reference))
  ;[0 0.8318 1] Begin Player & On interact
  (bind _asplayer_character_bp (Utilities|Casting|CastToPlayerCharacter_BP SourceCharacter))
  (bind _canberepaired_ (CallFunction|CanbeRepaired? _asplayer_character_bp))
  (if _canberepaired_
    (CallFunction|RepairItem _asplayer_character_bp)
    (Effects|SpawnEmitteratLocation (Variables|CustomSettings|GetSpecial%20Effect%20To%20Play) (Transformation|GetWorldLocation (Variables|Default|GetSFX-Location)))))

(event EventBeginPlay
  ;[0 0.8318 1] Begin Player & On interact
  (bind _returnvalue (UserInterface|CreateWidget "/Game/UI/WB_NotEnoughResources.WB_NotEnoughResources_C"))
  (Variables|Default|SetWIdgetReferenceNER _returnvalue))

(fn ConstructionScript)

(fn CanbeRepaired?
  (params (Player%20Reference :type Player%20Character%20BP%20Object%20Reference))
  (if (>= (Variables|/Game/MainFolder/PlayerFolder/PlayerBluePrints/PlayerCharacter_BP.PlayerCharacter_BP_C|GetWoodAmountCurrent Player%20Reference) (Variables|Default|GetWoodToRepair))
    (if (not (Variables|Default|GetHasBeenFixed?))
      (return true))
    (elif (not (Variables|Default|GetHasBeenFixed?))
      (UserInterface|Viewport|AddtoViewport (Variables|Default|GetWIdgetReferenceNER) 0)
      (return false))))

(fn RepairItem
  (params (NewParam :type Player%20Character%20BP%20Object%20Reference))
  (if (not (Variables|Default|GetHasBeenFixed?))
    (Variables|Default|SetHasBeenFixed? true)
    (Variables|/Game/MainFolder/PlayerFolder/PlayerBluePrints/PlayerCharacter_BP.PlayerCharacter_BP_C|SetWoodAmountCurrent NewParam (- (Variables|/Game/MainFolder/PlayerFolder/PlayerBluePrints/PlayerCharacter_BP.PlayerCharacter_BP_C|GetWoodAmountCurrent NewParam) (Variables|Default|GetWoodToRepair)))
    (Rendering|SetVisibility (Variables|Default|GetTextRender) false false)
    (if (Variables|CustomSettings|GetChangeMesh?)
      (Components|StaticMesh|SetStaticMesh (Variables|Character|GetMesh) (Variables|CustomSettings|GetNewMeshToChange)))
    (Collision|SetCollisionEnabled (Variables|Default|GetBoxCollision) "NoCollision")))