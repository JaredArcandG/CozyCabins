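; Repairable generator that the player fixes by interacting with it and spending EC resources.
; On interact, it checks the player's EC amount against the required cost, then deducts it once and flags itself repaired.
; Repair feedback turns on a spotlight, destroys the spark and smoke effects, and applies a green test material.
; With insufficient EC, a not-enough-resources widget created at BeginPlay is shown briefly, then removed.
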(event EventOnInteract
  (params (World :type World%20Object%20Reference) (SourceCharacter :type Character%20Object%20Reference))
  (bind _ner_reference (Variables|Default|GetNER%20Reference))
  ;[1 1 1] On interact we do a condition check if we have repaired generator
  (if (not (Variables|Default|GetHasRepaired?%20%28Generator%29))
    ;[1 1 1] if false we cast to player and check our resources
    (bind _asplayer_character_bp (Utilities|Casting|CastToPlayerCharacter_BP SourceCharacter))
    (if (>= (Variables|/Game/MainFolder/PlayerFolder/PlayerBluePrints/PlayerCharacter_BP.PlayerCharacter_BP_C|GetECAmountCurrent _asplayer_character_bp) (Variables|Default|GetEC-Required))
      ;[1 1 1] if we have the right amount we remove a set amount and set variable "repaired" to true
      (Utilities|FlowControl|DoOnce false
        (:Completed
          (Variables|/Game/MainFolder/PlayerFolder/PlayerBluePrints/PlayerCharacter_BP.PlayerCharacter_BP_C|SetECAmountCurrent _asplayer_character_bp (- (Variables|/Game/MainFolder/PlayerFolder/PlayerBluePrints/PlayerCharacter_BP.PlayerCharacter_BP_C|GetECAmountCurrent _asplayer_character_bp) (Variables|Default|GetEC-Required)))
          (Variables|Default|SetHasRepaired?%20%28Generator%29 true)
          ;[1 1 1] setting light above generator to "on" for feedback
          (Rendering|SetVisibility (Variables|Default|GetSpotlight) true false)
          ;[1 1 1] feedback
          (Components|DestroyComponent (Variables|Default|GetBlueprint_Effect_Sparks))
          ;[0 1 0.34] Debug
          (Rendering|Material|SetMaterial (Variables|Character|GetMesh) 0 "/Game/Art/Materials/TestMaterials/M_TestGreen.M_TestGreen")))
      (else
        ;[1 1 1] If false we display the correct widget
        (UserInterface|Viewport|AddtoViewport _ner_reference 0)
        (Utilities|FlowControl|Delay 2.0)
        (Widget|RemovefromParent _ner_reference)))))

(event EventBeginPlay
  ;[1 1 1] On Begin Play we set reference
  (bind _returnvalue (UserInterface|CreateWidget "/Game/UI/WB_NotEnoughResources.WB_NotEnoughResources_C"))
  (Variables|Default|SetNER%20Reference _returnvalue))

(fn ConstructionScript)