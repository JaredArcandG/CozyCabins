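; BpSwitch is an interactable switch that turns the repairable string lights on and off.
; On BeginPlay it caches a reference to the BPRepairStringLights actor found with GetActorOfClass.
; OnInteract checks that actor's generator-repaired and lights-repaired flags.
; When both are true, a FlipFlop alternates the visibility of its four light sources.
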(event EventBeginPlay
  ;[1 1 1] On Begin play we get the actor to gain acess to the variables inside instead of casting
  (Utilities|FlowControl|DoOnce false
    (:Completed
      (bind _returnvalue (Actor|GetActorOfClass "/Game/Blueprints/Repair/BP-RepairStringLights.BP-RepairStringLights_C"))
      (Variables|Default|SetSl-Reference _returnvalue))))

(event EventOnInteract
  (params (World :type World%20Object%20Reference) (SourceCharacter :type Character%20Object%20Reference))
  (bind _sl_reference (Variables|Default|GetSl-Reference))
  ;[1 1 1] On Interacting with the switch
  ;;[1 1 1] 2 Condition checks, one for checking if we repaired the generator and then the other for checking if we repaired the stringlights
  (if (Variables|/Game/Blueprints/Repair/BP-RepairStringLights.BP-RepairStringLights_C|GetHasRepairedGenerator? (Variables|Default|GetSl-Reference))
    (if (Variables|/Game/Blueprints/Repair/BP-RepairStringLights.BP-RepairStringLights_C|GetHasRepairedLIghts? (Variables|Default|GetSl-Reference))
      (Utilities|FlowControl|FlipFlop
        (:A
          ;;[1 1 1] Setting Visibility of the ligh sources on flip flops if we pass the condtion checks
          (Rendering|SetVisibility (Variables|/Game/Blueprints/Repair/BP-RepairStringLights.BP-RepairStringLights_C|GetLight1 _sl_reference) true false))
        (:B
          (Rendering|SetVisibility (Variables|/Game/Blueprints/Repair/BP-RepairStringLights.BP-RepairStringLights_C|GetLight4 _sl_reference) false false))))))

(fn ConstructionScript)