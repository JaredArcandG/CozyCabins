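; A repairable radio actor that the player fixes by spending their EC resource, then toggles music on and off.
; Interacting while broken checks the player's EC, then either deducts it, hides the text, spawns an effect and changes material or optional mesh, or shows a not-enough-resources widget.
; Once fixed, a FlipFlop starts or stops sound attached to the mesh.
; The sphere's end overlap removes the warning widget.
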(event OnComponentEndOverlap(Sphere)
  (params (OverlappedComponent :type Primitive%20Component%20Object%20Reference) (OtherActor :type Actor%20Object%20Reference) (OtherComp :type Primitive%20Component%20Object%20Reference) (OtherBodyIndex :type Integer))
  ;[0 0.8318 1] On interact
  (if (== OtherActor (Game|GetPlayerCharacter 0))
    (Widget|RemovefromParent (Variables|Default|GetWIdgetReferenceNER))))

(event EventOnInteract
  (params (World :type World%20Object%20Reference) (SourceCharacter :type Character%20Object%20Reference))
  (bind _mesh (Variables|Character|GetMesh))
  ;[0 0.8318 1] On interact
  ;;[1 1 1] Condition Check after interact - If True we run flip flop
  ;;
  ;; If False we run a player check
  (if (Variables|Default|GetHasBeenFixed?)
    (Utilities|FlowControl|FlipFlop
      (:A
        ;;[1 1 1] Spawn sound at the mesh location so it can move with the radio
        (bind _returnvalue (Audio|SpawnSoundAttached (Variables|Default|GetSound) _mesh "None" (Transformation|GetWorldLocation _mesh) "0, 0, 0" "KeepWorldPosition" false 0.4 1.0 0.0 0 0))
        (bind _output_get (Variables|Default|SetradioMusicReference _returnvalue))
        (Development|PrintString "Playing"))
      (:B
        ;;[1 1 1] Turning off when flipped to "B"
        (Audio|Components|Audio|Stop _output_get)
        (Development|PrintString "Stop")))
    (else
      ;;[1 1 1] Casting to player and checking if the object can be repaired
      ;; If we can repair we run the repair function and spawn VFX at location
      (bind _asplayer_character_bp (Utilities|Casting|CastToPlayerCharacter_BP SourceCharacter))
      (bind _canberepaired_ (CallFunction|CanbeRepaired? _asplayer_character_bp))
      (if _canberepaired_
        (CallFunction|RepairItem _asplayer_character_bp)
        (Effects|SpawnEmitteratLocation (Variables|CustomSettings|GetSpecial%20Effect%20To%20Play) (Transformation|GetWorldLocation (Variables|Default|GetSFX-Location)))
        ;;[1 1 1] Debug Color
        (Rendering|Material|SetMaterial (Variables|Character|GetMesh) 0 "/Game/Art/Materials/TestMaterials/M_Asparagus.M_Asparagus")))))

(event EventBeginPlay
  ;[0 1 0.9898] Begin play
  (bind _returnvalue (UserInterface|CreateWidget "/Game/UI/WB_NotEnoughResources.WB_NotEnoughResources_C"))
  (Variables|Default|SetWIdgetReferenceNER _returnvalue))

(fn ConstructionScript)

(fn CanbeRepaired?
  (params (Player%20Reference :type Player%20Character%20BP%20Object%20Reference))
  (if (>= (Variables|/Game/MainFolder/PlayerFolder/PlayerBluePrints/PlayerCharacter_BP.PlayerCharacter_BP_C|GetECAmountCurrent Player%20Reference) (Variables|Default|GetECToRepair))
    (if (not (Variables|Default|GetHasBeenFixed?))
      (return true))
    (elif (not (Variables|Default|GetHasBeenFixed?))
      (UserInterface|Viewport|AddtoViewport (Variables|Default|GetWIdgetReferenceNER) 0)
      (return false))))

(fn RepairItem
  (params (NewParam :type Player%20Character%20BP%20Object%20Reference))
  (if (not (Variables|Default|GetHasBeenFixed?))
    (Variables|Default|SetHasBeenFixed? true)
    (Variables|/Game/MainFolder/PlayerFolder/PlayerBluePrints/PlayerCharacter_BP.PlayerCharacter_BP_C|SetECAmountCurrent NewParam (- (Variables|/Game/MainFolder/PlayerFolder/PlayerBluePrints/PlayerCharacter_BP.PlayerCharacter_BP_C|GetECAmountCurrent NewParam) (Variables|Default|GetECToRepair)))
    (Rendering|SetVisibility (Variables|Default|GetTextRender) false false)
    (if (Variables|CustomSettings|GetChangeMesh?)
      (Components|StaticMesh|SetStaticMesh (Variables|Character|GetMesh) (Variables|CustomSettings|GetNewMeshToChange)))))