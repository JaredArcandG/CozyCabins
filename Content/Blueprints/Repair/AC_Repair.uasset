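; Actor component that lets the player repair a broken object using ingredients from their inventory.
; AttemptRepair resolves each ingredient's data table row, checks that the player's InventoryComponent holds strictly more than the required quantity, then removes the items and sets IsRepaired.
; GetRepairStatus exposes that flag, and ReturnRequiredText builds the "It's broken" message listing required amounts and item names.
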(event EventBeginPlay)

(event EventTick
  (params (DeltaSeconds :type Float%20%28single-precision%29)))

(fn AttemptRepair
  ;[1 1 1] Get Inventory if not valid
  (Utilities|IsValid (Variables|Default|GetInventory)
    (:Is%20Valid
      _)
    (:Is%20Not%20Valid
      (Variables|Default|SetInventory (Actor|GetComponentbyClass (Game|GetPlayerCharacter 0) "/Script/CozyCabinsGame.InventoryComponent"))))
  ;[1 1 1] Check if each required Ingredient exists in the Inventory and if enough Quantity is at Hand
  (for _array_element (Variables|Default|GetRepairIngredients)
    (bind _returnvalue (Utilities|GetDataTableRow (.DataTable (Utilities|Struct|BreakDataTableRowHandle (.ItemReference (Utilities|Struct|BreakCraftingItem _array_element)))) (.RowName (Utilities|Struct|BreakDataTableRowHandle (.ItemReference (Utilities|Struct|BreakCraftingItem _array_element)))))
      (:then
        (bind (_resultdata _quantity _returnvalue_2) (Class|InventoryComponent|TryGetItem (Variables|Default|GetInventory) (.Id (Utilities|Struct|BreakItemData _returnvalue))))
        (if (not (and _returnvalue_2 (> _quantity (.Quantity (Utilities|Struct|BreakCraftingItem _array_element)))))
          ;[1 1 1] Insufficient Items
          (return false)))))
  ;[1 1 1] Consume Items
  (for _array_element_2 (Variables|Default|GetRepairIngredients)
    (bind _returnvalue_3 (Utilities|GetDataTableRow (.DataTable (Utilities|Struct|BreakDataTableRowHandle (.ItemReference (Utilities|Struct|BreakCraftingItem _array_element_2)))) (.RowName (Utilities|Struct|BreakDataTableRowHandle (.ItemReference (Utilities|Struct|BreakCraftingItem _array_element_2)))))
      (:then
        (bind _returnvalue_4 (Class|InventoryComponent|TryRemove (Variables|Default|GetInventory) (.Id (Utilities|Struct|BreakItemData _returnvalue_3)) (.Quantity (Utilities|Struct|BreakCraftingItem _array_element_2))))
        (if (not _returnvalue_4)
          ;[1 1 1] Error removing Items
          (return false)))))
  ;[1 1 1] Set Repaired to true
  (Variables|Default|SetIsRepaired true)
  (return true))

(fn GetRepairStatus
  (return (Variables|Default|GetIsRepaired)))

(fn ReturnRequiredText
  (for _array_element (Variables|Default|GetRepairIngredients)
    (bind _returnvalue (Utilities|GetDataTableRow (.DataTable (Utilities|Struct|BreakDataTableRowHandle (.ItemReference (Utilities|Struct|BreakCraftingItem _array_element)))) (.RowName (Utilities|Struct|BreakDataTableRowHandle (.ItemReference (Utilities|Struct|BreakCraftingItem _array_element)))))
      (:then
        (Utilities|Array|Add (LocalVariables|GetRequiredItems) (Utilities|String|ToString(Text) (Utilities|Text|FormatText "{Amount}x {Name}" (.Quantity (Utilities|Struct|BreakCraftingItem _array_element)) (.Name (Utilities|Struct|BreakItemData _returnvalue))))))))
  (return (Utilities|Text|FormatText "It's broken.  
To repair you need: 
{Items}" (Utilities|String|JoinStringArray (LocalVariables|GetRequiredItems) " 
"))))