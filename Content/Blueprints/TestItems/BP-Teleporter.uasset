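; BP-Teleporter is a test-item teleporter actor that relocates the player character when it enters one of two trigger capsules.
; Overlapping Capsule1 moves the player to the world location of component 1, and Capsule2 does the same with component 2.
; Each overlap casts to PlayerCharacter_BP, ignoring other actors, then sets the capsule component's location directly, without sweep or teleport physics.
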(event OnComponentBeginOverlap(Capsule1)
  (params (OverlappedComponent :type Primitive%20Component%20Object%20Reference) (OtherActor :type Actor%20Object%20Reference) (OtherComp :type Primitive%20Component%20Object%20Reference) (OtherBodyIndex :type Integer) (bFromSweep :type Boolean) (SweepResult :type Hit%20Result%20Structure%20%28by%20ref%29))
  (bind _asplayer_character_bp (Utilities|Casting|CastToPlayerCharacter_BP OtherActor))
  (Transformation|SetWorldLocation (Variables|/Script/Engine.Character|GetCapsuleComponent _asplayer_character_bp) (Transformation|GetWorldLocation (Variables|Default|Get1)) false false))

(event OnComponentBeginOverlap(Capsule2)
  (params (OverlappedComponent :type Primitive%20Component%20Object%20Reference) (OtherActor :type Actor%20Object%20Reference) (OtherComp :type Primitive%20Component%20Object%20Reference) (OtherBodyIndex :type Integer) (bFromSweep :type Boolean) (SweepResult :type Hit%20Result%20Structure%20%28by%20ref%29))
  (bind _asplayer_character_bp (Utilities|Casting|CastToPlayerCharacter_BP OtherActor))
  (Transformation|SetWorldLocation (Variables|/Script/Engine.Character|GetCapsuleComponent _asplayer_character_bp) (Transformation|GetWorldLocation (Variables|Default|Get2)) false false))

(event EventBeginPlay)

(event Collision|EventActorBeginOverlap
  (params (OtherActor :type Actor%20Object%20Reference)))

(event EventTick
  (params (DeltaSeconds :type Float%20%28single-precision%29)))

(fn ConstructionScript)