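; BP_TestItemB is a test item actor that the player can pick up into an inventory.
; On interact, it casts the source to PlayerCharacter and tries to add its data ID and quantity to that character's inventory component, destroying itself on success.
; Its OnUse override only prints a consumption message and returns false.
; Debug prints mark the interaction and successful add.
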(event EventBeginPlay)

(event Collision|EventActorBeginOverlap
  (params (OtherActor :type Actor%20Object%20Reference)))

(event EventTick
  (params (DeltaSeconds :type Float%20%28single-precision%29)))

(event EventOnInteract
  (params (World :type World%20Object%20Reference) (SourceCharacter :type Character%20Object%20Reference))
  (Development|PrintString "Interact called on test item b. Adding to inventory.")
  (bind _asplayer_character (Utilities|Casting|CastToPlayerCharacter SourceCharacter))
  (bind _returnvalue (Class|PlayerCharacter|GetInventoryComponent _asplayer_character))
  (Utilities|IsValid _returnvalue
    (:Is%20Valid
      (bind _returnvalue_2 (Class|Item|GetData))
      (bind _returnvalue_3 (Class|InventoryComponent|TryAdd _returnvalue (.Id (Utilities|Struct|BreakItemData _returnvalue_2)) (Variables|Default|GetQuantity)))
      (if _returnvalue_3
        (Development|PrintString "ItemAddedSucessfully")
        (Actor|DestroyActor)))))

(fn ConstructionScript)

(fn OnUse
  (params (World :type World%20Object%20Reference) (SourceCharacter :type Character%20Object%20Reference))
  (Development|PrintString "Consumed Test Item B Successfully!")
  (return false))