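; Dandelion consumable pickup that adds to the character's dandelion count.
; It overrides the parent's Pickup event to increase the current amount, print debug messages and then run the parent logic.
; Its CanBePickedUp check calls the parent version, ignores that result, and refuses pickup when the amount to add would exceed the character's maximum.
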(event EventPickup
  (params (Charcter :type Player%20Character%20BP%20Object%20Reference))
  (bind _output_get (Variables|/Game/MainFolder/PlayerFolder/PlayerBluePrints/PlayerCharacter_BP.PlayerCharacter_BP_C|SetDandelionAmountCurrent Charcter (+ (Variables|/Game/MainFolder/PlayerFolder/PlayerBluePrints/PlayerCharacter_BP.PlayerCharacter_BP_C|GetDandelionAmountCurrent Charcter) (Variables|Default|GetDandelionToAdd))))
  (Development|PrintString "Dandelion Picked Up")
  (Development|PrintString (Utilities|String|ToString(Float) _output_get))
  (|CallParentFunction Charcter))

(fn ConstructionScript
  (|CallParentFunction))

(fn CanbePickedUp?
  (params (Character :type Player%20Character%20BP%20Object%20Reference))
  (|CallParentFunction Character)
  (if (> (+ (Variables|/Game/MainFolder/PlayerFolder/PlayerBluePrints/PlayerCharacter_BP.PlayerCharacter_BP_C|GetDandelionAmountCurrent Character) (Variables|Default|GetDandelionToAdd)) (Variables|/Game/MainFolder/PlayerFolder/PlayerBluePrints/PlayerCharacter_BP.PlayerCharacter_BP_C|GetDandelionAmountMax Character))
    (return false)
    (else
      (return true))))