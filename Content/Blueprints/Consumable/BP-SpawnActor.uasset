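; Consumable respawner Blueprint that spawns a replacement actor of a chosen class after a delay.
; On BeginPlay it caches the first actor found of that class.
; StartTimer sets a timer to RespawnActor, which spawns the cached actor's class at that actor's current root transform and clears the timer.
; The picked-up dispatcher binding is never executed, and nothing in this graph calls StartTimer.
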(event Custom|StartTimer
  (bind _returnvalue (Utilities|Time|SetTimerbyEvent (delegate Custom|RespawnActor) (Variables|Custom|GetTimeToRespawn))))

(event Custom|RespawnActor
  (Game|SpawnActorfromClass (Utilities|GetClass (stale EventBeginPlay _returnvalue)) (Math|Transform|MakeTransform (Transformation|GetWorldLocation (Variables|/Script/Engine.Actor|GetRootComponent (stale EventBeginPlay _returnvalue))) (Transformation|GetWorldRotation (Variables|/Script/Engine.Actor|GetRootComponent (stale EventBeginPlay _returnvalue))) "1.000000,1.000000,1.000000") "Undefined" "MultiplyWithRoot" 0 0)
  (Utilities|Time|ClearandInvalidateTimerbyHandle (stale Custom|StartTimer _returnvalue)))

(event EventBeginPlay
  (bind _returnvalue (Actor|GetActorOfClass (Variables|Default|GetClass)))
  (Actor|GetActorOfClass 0))

(fn ConstructionScript)