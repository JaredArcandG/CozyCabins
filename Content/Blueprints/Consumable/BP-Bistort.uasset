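; Consumable pickup Blueprint for Bistort that adds to the collecting character's Bistort count.
; It overrides a parent pickup class: Pickup adds BistortToAdd to the character's current amount, prints debug messages with the new total, then calls the parent Pickup.
; CanBePickedUp refuses the pickup when adding that amount would exceed the character's Bistort maximum, ignoring the parent's result.
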(event EventPickup
  (params (Charcter :type Player%20Character%20BP%20Object%20Reference))
  (bind _output_get (Variables|/Game/MainFolder/PlayerFolder/PlayerBluePrints/PlayerCharacter_BP.PlayerCharacter_BP_C|SetBistortAmountCurrent Charcter (+ (Variables|/Game/MainFolder/PlayerFolder/PlayerBluePrints/PlayerCharacter_BP.PlayerCharacter_BP_C|GetBistortAmountCurrent Charcter) (Variables|Default|GetBistortToAdd))))
  (Development|PrintString "Bistort Picked Up")
  (Development|PrintString (Utilities|String|ToString(Float) _output_get))
  (|CallParentFunction Charcter))

(fn ConstructionScript
  (|CallParentFunction))

(fn CanbePickedUp?
  (params (Character :type Player%20Character%20BP%20Object%20Reference))
  (|CallParentFunction Character)
  (if (> (+ (Variables|/Game/MainFolder/PlayerFolder/PlayerBluePrints/PlayerCharacter_BP.PlayerCharacter_BP_C|GetBistortAmountCurrent Character) (Variables|Default|GetBistortToAdd)) (Variables|/Game/MainFolder/PlayerFolder/PlayerBluePrints/PlayerCharacter_BP.PlayerCharacter_BP_C|GetBistortAmountMax Character))
    (return false)
    (else
      (return true))))