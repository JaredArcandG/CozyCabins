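; BPBasePickup is a base pickup actor that a player character collects by interacting with it.
; OnInteract casts the source to PlayerCharacter_BP and calls Pickup only if CanBePickedUp allows it, which returns false here as an apparent override point.
; Pickup plays a 2D sound and destroys the actor.
; Each tick, a TextRender component turns to face the player camera, under a "Testing" comment.
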(event Custom|Pickup
  (params (Charcter :type Player%20Character%20BP%20Object%20Reference))
  (Audio|PlaySound2D (Variables|Default|GetPickupSound) 1.0 1.0 0.0 0 0)
  (Actor|DestroyActor))

(event EventTick
  (params (DeltaSeconds :type Float%20%28single-precision%29))
  (bind _textrender (Variables|Default|GetTextRender))
  ;[0 0.8713 1] Testing
  (Transformation|SetWorldRotation _textrender (Math|Rotator|FindLookatRotation (Transformation|GetWorldLocation _textrender) (Transformation|GetWorldLocation (Variables|/Script/Engine.PlayerCameraManager|GetTransformComponent (Game|GetPlayerCameraManager 0)))) false false))

(event EventOnInteract
  (params (World :type World%20Object%20Reference) (SourceCharacter :type Character%20Object%20Reference))
  (bind _asplayer_character_bp (Utilities|Casting|CastToPlayerCharacter_BP SourceCharacter))
  (bind _can_be_picked_up_ (CallFunction|CanbePickedUp? _asplayer_character_bp))
  (if _can_be_picked_up_
    (CallFunction|Pickup _asplayer_character_bp)))

(fn ConstructionScript)

(fn CanbePickedUp?
  (params (Character :type Player%20Character%20BP%20Object%20Reference))
  (return false))